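; NPC AI controller that runs a guard behavior tree and feeds it perceived targets.
; On BeginPlay it sets up the Patrol_Data blackboard and starts GuardBehavior.
; Perception updates for actors without the "Enemy" tag write the actor to the enemy blackboard key when sensed, and clear that key when sensing is lost.
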(event OnTargetPerceptionUpdated(AIPerception)
  (params (Actor :type Actor%20Object%20Reference) (Stimulus :type AI%20Stimulus%20Structure))
  (CallFunction|UpdateBlackboardEnemyKey Actor Stimulus Actor))

(event EventBeginPlay
  (bind _blackboardcomponent (Class|AIController|UseBlackboard "/Game/Dynamic/Character/AI/Patrol_Data.Patrol_Data"))
  (AI|RunBehaviorTree "/Game/Dynamic/Character/AI/GuardBehavior.GuardBehavior")
  (Variables|Default|SetBlackboard%20Component _blackboardcomponent))

(fn ConstructionScript)

(fn UpdateBlackboardEnemyKey
  (params (ObjectValue :type Object%20Object%20Reference) (AIStimulus :type AI%20Stimulus%20Structure%20%28by%20ref%29) (Check%20Actor%20Tag :type Actor%20Object%20Reference))
  (bind _enemy_key (Variables|Default|GetEnemy%20Key))
  (bind _blackboard_component (Variables|Default|GetBlackboard%20Component))
  (if (not (Actor|ActorHasTag Check%20Actor%20Tag "Enemy"))
    (if (.bSuccessfullySensed (Utilities|Struct|BreakAIStimulus AIStimulus))
      (AI|Components|Blackboard|SetValueasObject _blackboard_component _enemy_key ObjectValue)
      (else
        (AI|Components|Blackboard|ClearValue _blackboard_component _enemy_key)))))