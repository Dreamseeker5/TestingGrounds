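; NPC AI controller that runs the GuardBehavior behavior tree with the Patrol_Data blackboard on its pawn.
; AI perception writes sensed actors lacking the "Enemy" tag to the blackboard's enemy key and clears it when such an actor's sensing fails.
; Each tick, it sets the controlled TP_Character's aiming and firing flags according to whether the controller has a valid focus actor.
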(event OnTargetPerceptionUpdated(AIPerception)
  (params (Actor :type Actor%20Object%20Reference) (Stimulus :type AI%20Stimulus%20Structure))
  (bind _blackboard_component (Variables|Default|GetBlackboard%20Component))
  (bind _enemy_key (Variables|Default|GetEnemy%20Key))
  (if (not (Actor|ActorHasTag Actor "Enemy"))
    (if (.bSuccessfullySensed (Utilities|Struct|BreakAIStimulus Stimulus))
      (AI|Components|Blackboard|SetValueasObject _blackboard_component _enemy_key Actor)
      (else
        (AI|Components|Blackboard|ClearValue _blackboard_component _enemy_key)))))

(event EventBeginPlay
  (bind _blackboardcomponent (Class|AIController|UseBlackboard "/Game/Dynamic/NPC/AI/Patrol_Data.Patrol_Data"))
  (AI|RunBehaviorTree "/Game/Dynamic/NPC/AI/GuardBehavior.GuardBehavior")
  (Variables|Default|SetBlackboard%20Component _blackboardcomponent))

(event EventTick
  (params (DeltaSeconds :type Float%20%28single-precision%29))
  (bind _returnvalue (Class|AIController|GetFocusActor))
  (bind _returnvalue_2 (Utilities|IsValid _returnvalue))
  (bind _astp_character (Utilities|Casting|CastToTP_Character (Pawn|GetControlledPawn)))
  (Variables|/Game/Dynamic/NPC/Behavior/TP_Character.TP_Character_C|SetIsAiming _astp_character _returnvalue_2)
  (Variables|/Game/Dynamic/NPC/Behavior/TP_Character.TP_Character_C|SetIsFiring _astp_character _returnvalue_2))

(fn ConstructionScript)